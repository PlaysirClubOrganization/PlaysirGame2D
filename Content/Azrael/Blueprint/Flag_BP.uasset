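; Level-end flag actor that completes the level when the AlienHero_BP character overlaps it.
; On overlap it calls LevelSuceed, which proceeds only if the hero's Lock flag is true.
; It copies the hero's coin count and incremented level number into the hero's Saver object and writes it to the "SaveGame" slot.
; It then always opens the map "Level1", whatever level number was saved.
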(event EventBeginPlay)

(event EventActorBeginOverlap
  (params (OtherActor :type Actor%20Object%20Reference))
  (if (== (Utilities|GetClass OtherActor) "/Game/Azrael/Gameplay/AlienHero_BP.AlienHero_BP_C")
    (CallFunction|LevelSuceed (.AsAlien%20Hero%20BP (Utilities|Casting|CastToAlienHero_BP OtherActor)))))

(event EventTick
  (params (DeltaSeconds :type Float%20%28single-precision%29)))

(fn ConstructionScript)

(fn LevelSuceed
  (params (Character :type Alien%20Hero%20BP%20Object%20Reference))
  (bind _saver (Variables|/Game/Azrael/Gameplay/AlienHero_BP.AlienHero_BP_C|GetSaver Character))
  (if (Variables|/Game/Azrael/Gameplay/AlienHero_BP.AlienHero_BP_C|GetLock Character)
    (Variables|/Game/Azrael/Gameplay/BP_SaveGame.BP_SaveGame_C|SetCount _saver (Variables|/Game/Azrael/Gameplay/AlienHero_BP.AlienHero_BP_C|GetCountCoin Character))
    (Variables|/Game/Azrael/Gameplay/BP_SaveGame.BP_SaveGame_C|SetLevel _saver (+ (Variables|/Game/Azrael/Gameplay/AlienHero_BP.AlienHero_BP_C|GetLevel Character) 1))
    (SaveGame|SaveGametoSlot _saver "SaveGame")
    (Game|OpenLevel(byName) "Level1"))
  (return))
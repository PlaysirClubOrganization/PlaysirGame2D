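; BP_Enemy is a basic enemy, marked as a TODO, that patrols and threatens the player on contact.
; When its AI flag is set, BeginPlay starts an endless latent MoveComponentTo loop that eases the root between the TargetAller and TargetRetour actor locations.
; Actor overlap destroys it when hit by BP_Projectile, or opens Level0 when it touches AlienHero_BP.
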(event EventBeginPlay
  (bind _defaultsceneroot (Variables|Default|GetDefaultSceneRoot))
  ;[1 1 1] TODO : basic Enemy
  (if (Variables|Default|GetAI)
    (Components|MoveComponentTo _defaultsceneroot (Transformation|GetActorLocation (Variables|Default|GettargetAller)) "0, 0, 0" false true 2.0 :!label _label)
    (Components|MoveComponentTo _defaultsceneroot (Transformation|GetActorLocation (Variables|Default|GettargetRetour)) "0, 0, 0" false true 2.0)
    (goto _label)))

(event EventActorBeginOverlap
  (params (OtherActor :type Actor%20Object%20Reference))
  ;[1 1 1] TODO : basic Enemy
  (if (== (Utilities|GetClass OtherActor) "/Game/Azrael/Blueprint/BP_Projectile.BP_Projectile_C")
    (Actor|DestroyActor))
  (if (== (Utilities|GetClass OtherActor) "/Game/Azrael/Gameplay/AlienHero_BP.AlienHero_BP_C")
    (Game|OpenLevel(byName) "Level0")))

(event EventTick
  (params (DeltaSeconds :type Float%20%28single-precision%29))
  ;[1 1 1] TODO : basic Enemy
)

(fn ConstructionScript
  (|CallParentFunction))
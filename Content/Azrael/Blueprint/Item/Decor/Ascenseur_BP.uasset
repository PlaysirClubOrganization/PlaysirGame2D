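; Elevator decor item that carries the AlienHero character upward while it is inside a Box trigger.
; On begin overlap, it switches the hero's movement to Flying and sets a strong upward velocity.
; On end overlap, it returns the hero to Falling with a smaller upward boost.
; The lift works purely through character movement changes, with no Tick or timeline logic.
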(event OnComponentEndOverlap(Box)
  (params (OtherActor :type Actor%20Object%20Reference) (OtherComp :type Primitive%20Component%20Object%20Reference) (OtherBodyIndex :type Integer))
  (bind _asalien_hero_bp (Utilities|Casting|CastToAlienHero_BP OtherActor))
  (Pawn|Components|CharacterMovement|SetMovementMode (Variables|/Script/Engine.Character|GetCharacterMovement _asalien_hero_bp) "MOVE_Falling" 0)
  (Variables|/Script/Engine.MovementComponent|SetVelocity (Variables|/Script/Engine.Character|GetCharacterMovement _asalien_hero_bp) "0, 0,250.000000"))

(event OnComponentBeginOverlap(Box)
  (params (OtherActor :type Actor%20Object%20Reference) (OtherComp :type Primitive%20Component%20Object%20Reference) (OtherBodyIndex :type Integer) (bFromSweep :type Boolean) (SweepResult :type Hit%20Result%20Structure%20%28by%20ref%29))
  (bind _asalien_hero_bp (Utilities|Casting|CastToAlienHero_BP OtherActor))
  (Pawn|Components|CharacterMovement|SetMovementMode (Variables|/Script/Engine.Character|GetCharacterMovement _asalien_hero_bp) "MOVE_Flying" 0)
  (Variables|/Script/Engine.MovementComponent|SetVelocity (Variables|/Script/Engine.Character|GetCharacterMovement _asalien_hero_bp) "0, 0,800.000000"))

(event EventBeginPlay)

(event EventTick
  (params (DeltaSeconds :type Float%20%28single-precision%29)))

(fn ConstructionScript
  (|CallParentFunction))
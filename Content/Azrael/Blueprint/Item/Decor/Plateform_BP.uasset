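; Decor platform Blueprint with a resizable collision component and two extremity markers, ExtremA and ExtremB.
; The construction script multiplies the collision's X and Z scale by SizeX and SizeZ, with Y fixed.
; BeginPlay caches both markers' world locations in variables; no movement or overlap logic is implemented in these graphs.
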(event EventBeginPlay
  (Variables|Default|SetlocationExtremityA (Transformation|GetWorldLocation (Variables|Default|GetExtremA)))
  (Variables|Default|SetlocationExtremityB (Transformation|GetWorldLocation (Variables|Default|GetExtremB))))

(event EventActorBeginOverlap
  (params (OtherActor :type Actor%20Object%20Reference)))

(event EventTick
  (params (DeltaSeconds :type Float%20%28single-precision%29)))

(fn ConstructionScript
  (bind _platformcollision (Variables|Default|GetPlatFormCollision))
  (bind _relativescale3d (Variables|/Script/Engine.SceneComponent|GetRelativeScale3D _platformcollision))
  (Transformation|SetRelativeScale3D _platformcollision (Math|Vector|MakeVector (* (Variables|Default|GetSizeX) (.x _relativescale3d)) 0.5 (* (.z _relativescale3d) (Variables|Default|GetSizeZ)))))
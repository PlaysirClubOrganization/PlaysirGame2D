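; Extendable decor platform that builds a grid of Paper2D sprites in its construction script, sized by Longueur (length) and Hauteur (height).
; Two arrow components set the horizontal and vertical step relative to the base sprite, and running offsets place each added sprite.
; HorizontalCreation fills each row with middle sprites and a right cap after the left-end sprite.
; Color tints only the base sprite, as the SetSpriteColor pass over added sprites never runs.
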(event EventBeginPlay)

(event EventActorBeginOverlap
  (params (OtherActor :type Actor%20Object%20Reference))
  (|CallParentFunction 0))

(event EventTick
  (params (DeltaSeconds :type Float%20%28single-precision%29)))

(fn ConstructionScript
  (bind _papersprite (Variables|Default|GetPaperSprite))
  (Rendering|Components|Sprite|SetSprite _papersprite (Variables|Default|GetGaucheS))
  (Sprite|SetSpriteColor _papersprite (Variables|Default|GetColor))
  (Variables|Default|SetInsertPointH (- (Variables|/Script/Engine.SceneComponent|GetRelativeLocation (Variables|Default|GetArrow)) (Variables|/Script/Engine.SceneComponent|GetRelativeLocation (Variables|Default|GetPaperSprite))))
  (Variables|Default|SetInsertPointV (- (Variables|/Script/Engine.SceneComponent|GetRelativeLocation (Variables|Default|GetArrow1)) (Variables|/Script/Engine.SceneComponent|GetRelativeLocation (Variables|Default|GetPaperSprite))))
  (Utilities|HorizontalCreation)
  (for _index (range 1 (- (Variables|Default|GetHauteur) 1))
    (bind _returnvalue (AddComponent|AddPaperSpriteComponent false (Math|Conversions|ToTransform(Vector) (+ (Variables|Default|GetInsertPointV) (Variables|Default|GetMemoryV)))))
    (Utilities|AddSpriteComponent _returnvalue)
    (Variables|Default|SetMemoryV (Variables|/Script/Engine.SceneComponent|GetRelativeLocation _returnvalue))
    (Rendering|Components|Sprite|SetSprite _returnvalue (Variables|Default|GetGaucheS))
    (Variables|Default|SetMemoryH (Variables|Default|GetMemoryV))
    (Utilities|HorizontalCreation))
  (Utilities|SetSpriteColor
    (:execute2
      (|CallParentFunction))))
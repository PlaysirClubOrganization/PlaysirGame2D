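; Activator_BP is a one-shot switch that the player triggers with F to activate extending platforms.
; Capsule overlap with AlienHero_BP toggles input for player controller 0 and tracks whether the hero is in range.
; On F, it prints a debug "Hello", then if in range and still usable calls Activation on each Plateform_extend_BP_Child in ElementsActive and clears CanActivate.
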(event OnComponentBeginOverlap(Capsule)
  (params (OtherActor :type Actor%20Object%20Reference) (OtherComp :type Primitive%20Component%20Object%20Reference) (OtherBodyIndex :type Integer) (bFromSweep :type Boolean) (SweepResult :type Hit%20Result%20Structure%20%28by%20ref%29))
  (Utilities|Casting|CastToAlienHero_BP OtherActor)
  (Input|EnableInput (Game|GetPlayerController 0))
  (Variables|Default|SetisOverlaping true))

(event OnComponentEndOverlap(Capsule)
  (params (OtherActor :type Actor%20Object%20Reference) (OtherComp :type Primitive%20Component%20Object%20Reference) (OtherBodyIndex :type Integer))
  (Utilities|Casting|CastToAlienHero_BP OtherActor)
  (Input|DisableInput (Game|GetPlayerController 0))
  (Variables|Default|SetisOverlaping false))

(event EventBeginPlay)

(event Input|KeyboardEvents|F
  (params (Key :type Key%20Structure :default "AnyKey"))
  (:Pressed
    (Development|PrintString "Hello")
    (Utilities|Casting|CastToAlienHero_BP (Game|Player|GetPlayerPawn 0))
    (if (and (Variables|Default|GetcanActivate) (Variables|Default|GetisOverlaping))
      (for _array_element (Variables|Default|GetElementsActive)
        (bind _asplateform_extend_bp_child (Utilities|Casting|CastToPlateform_extend_BP_Child _array_element))
        (Default|Activation _asplateform_extend_bp_child))
      (Variables|Default|SetcanActivate false))))

(fn ConstructionScript
  (|CallParentFunction))
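; A decor platform actor that travels endlessly through a list of destination points.
; The construction script stores the actor's location as Origin, so each entry in Destinations acts as an offset from that placement.
; From BeginPlay, a latent MoveComponentTo moves the root component to each point over Duration, then advances a wrapping index and loops back, without using Tick.
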(event EventBeginPlay
  (Components|MoveComponentTo (Variables|Default|GetDefaultSceneRoot) (+ (Utilities|Array|Get(acopy) (Variables|Default|GetDestinations) (Variables|Default|GetLoopMem)) (Variables|Default|GetOrigin)) "0, 0, 0" false false (Variables|Default|GetDuration) :!label _label)
  (Variables|Default|SetLoopMem (Math|Integer|%(Integer) (+ (Variables|Default|GetLoopMem) 1) (Utilities|Array|Length (Variables|Default|GetDestinations))))
  (goto _label))

(event EventActorBeginOverlap
  (params (OtherActor :type Actor%20Object%20Reference))
  (|CallParentFunction 0))

(event EventTick
  (params (DeltaSeconds :type Float%20%28single-precision%29)))

(fn ConstructionScript
  (|CallParentFunction)
  (Variables|Default|SetOrigin (Transformation|GetActorLocation)))
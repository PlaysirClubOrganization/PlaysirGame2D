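; Projectile actor with a sprite that travels horizontally along the world X axis.
; Every Tick it offsets its X location by a fixed step times the Direction variable, without delta-time scaling or sweep.
; Logic that would derive Direction from the sprite's yaw is disconnected in the construction script, so Direction is not set here.
; No overlap, damage or lifetime handling is implemented.
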(event EventBeginPlay)

(event EventActorBeginOverlap
  (params (OtherActor :type Actor%20Object%20Reference)))

(event EventTick
  (params (DeltaSeconds :type Float%20%28single-precision%29))
  (bind _returnvalue (Transformation|GetActorLocation))
  (Transformation|SetActorLocation (Math|Vector|MakeVector (+ (* (Variables|Default|Getdirection) 12.0) (.x _returnvalue)) (.y _returnvalue) (.z _returnvalue)) false false))

(fn ConstructionScript)
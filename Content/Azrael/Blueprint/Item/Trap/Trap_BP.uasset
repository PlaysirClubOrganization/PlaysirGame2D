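; Trap actor that deals its Damage value to any AbstractPlayer that overlaps it.
; The construction script picks the Paper2D sprite from the trap Type, with only the Spike case handled.
; A ReloadCurrentLevel helper opens the level named from the saved level number on the player's AlienHero_BP pawn, but nothing in this file calls it.
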(event EventBeginPlay)

(event EventActorBeginOverlap
  (params (OtherActor :type Actor%20Object%20Reference))
  (bind (_asabstract_player _bsuccess) (Utilities|Casting|CastToAbstractPlayer OtherActor))
  (|CallParentFunction OtherActor)
  (if _bsuccess
    (Class|AbstractPlayer|TakeDamages _asabstract_player (Variables|Default|Getdamage))))

(event EventTick
  (params (DeltaSeconds :type Float%20%28single-precision%29)))

(fn ConstructionScript
  (|CallParentFunction)
  (switch Utilities|FlowControl|Switch|SwitchonItem_Trap (Variables|Default|Gettype)
    (:Spike
      (Rendering|Components|Sprite|SetSprite (Variables|Default|GetPaperSprite) "/Game/KenneySpritePack/Tiles/spikes_Sprite.spikes_Sprite"))))

(fn ReloadCurrentLevel
  (Game|OpenLevel(byName) (Utilities|String|StringToName (Utilities|String|Append "Level" (Utilities|String|ToString(Integer) (Variables|/Game/Azrael/Gameplay/BP_SaveGame.BP_SaveGame_C|GetLevel (Variables|/Game/Azrael/Gameplay/AlienHero_BP.AlienHero_BP_C|GetSaver (.AsAlien%20Hero%20BP (Utilities|Casting|CastToAlienHero_BP (Game|Player|GetPlayerPawn 0)))))))))
  (return))
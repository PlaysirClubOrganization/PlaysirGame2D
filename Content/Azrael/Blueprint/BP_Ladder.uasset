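; BP_Ladder is a ladder actor that marks where the AlienHero_BP character is allowed to climb.
; Entering its Box trigger sets the hero's CanClimb flag, leaving the climbing behavior itself outside this Blueprint.
; Leaving the box clears CanClimb and IsClimbing, restores the sprite's normal play rate and switches character movement to Falling.
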(event OnComponentBeginOverlap(Box)
  (params (OtherActor :type Actor%20Object%20Reference) (OtherComp :type Primitive%20Component%20Object%20Reference) (OtherBodyIndex :type Integer) (bFromSweep :type Boolean) (SweepResult :type Hit%20Result%20Structure%20%28by%20ref%29))
  ;[1 1 1] Enabling - Desabling climb action
  (bind _asalien_hero_bp (Utilities|Casting|CastToAlienHero_BP OtherActor))
  (Variables|/Game/Azrael/Gameplay/AlienHero_BP.AlienHero_BP_C|SetcanClimb _asalien_hero_bp true))

(event OnComponentEndOverlap(Box)
  (params (OtherActor :type Actor%20Object%20Reference) (OtherComp :type Primitive%20Component%20Object%20Reference) (OtherBodyIndex :type Integer))
  ;[1 1 1] Enabling - Desabling climb action
  (bind _asalien_hero_bp (Utilities|Casting|CastToAlienHero_BP OtherActor))
  (Components|Timeline|SetPlayRate (Variables|/Script/Paper2D.PaperCharacter|GetSprite _asalien_hero_bp) 1.0)
  (Variables|/Game/Azrael/Gameplay/AlienHero_BP.AlienHero_BP_C|SetcanClimb _asalien_hero_bp false)
  (Variables|/Game/Azrael/Gameplay/AlienHero_BP.AlienHero_BP_C|SetisClimbing _asalien_hero_bp false)
  (Pawn|Components|CharacterMovement|SetMovementMode (Variables|/Script/Engine.Character|GetCharacterMovement _asalien_hero_bp) "MOVE_Falling" 0))

(event EventBeginPlay)

(event EventActorBeginOverlap
  (params (OtherActor :type Actor%20Object%20Reference))
  (|CallParentFunction 0))

(event EventTick
  (params (DeltaSeconds :type Float%20%28single-precision%29)))

(fn ConstructionScript
  (|CallParentFunction))
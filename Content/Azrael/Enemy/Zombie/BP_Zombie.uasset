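; Flipbook-sprite zombie enemy that plays an appear phase on spawn, then idles until pawn sensing sees a pawn.
; A sighting sets a flipbook and drives it along world +X by overriding velocity unless falling, while hearing only prints debug text.
; DetectorJump triggers a forward jump at BP_Item_Destroyed_Character overlaps, and Detector triggers a jump when an overlap ends without a detected trap.
; Construction calls InitEnemy.
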(event OnComponentBeginOverlap(DetectorJump)
  (params (OtherActor :type Actor%20Object%20Reference) (OtherComp :type Primitive%20Component%20Object%20Reference) (OtherBodyIndex :type Integer) (bFromSweep :type Boolean) (SweepResult :type Hit%20Result%20Structure%20%28by%20ref%29))
  (bind _charactermovement (Variables|Character|GetCharacterMovement))
  (bind _output_get (Variables|Default|SettrapDetected (.bSuccess (Utilities|Casting|CastToBP_Item_Destroyed_Character OtherActor))))
  (if _output_get
    (Development|PrintString "Detector Jumb" true true "(R=1.000000,G=0.000000,B=0.074743,A=1.000000)")
    (Character|Jump)
    (Sprite|SetFlipbook (Variables|Default|GetSprite) "/Game/Azrael/Enemy/Zombie/FlipBook/idle.idle")
    (Variables|/Script/Engine.MovementComponent|SetVelocity _charactermovement (Math|Vector|MakeVector 2.5e+02 0.0 (.z (Variables|/Script/Engine.MovementComponent|GetVelocity _charactermovement))))))

(event OnComponentEndOverlap(Detector)
  (params (OtherActor :type Actor%20Object%20Reference) (OtherComp :type Primitive%20Component%20Object%20Reference) (OtherBodyIndex :type Integer))
  (bind _charactermovement (Variables|Character|GetCharacterMovement))
  (if (not (Variables|Default|GettrapDetected))
    (Character|Jump)
    (Variables|/Script/Engine.MovementComponent|SetVelocity _charactermovement (+ (Variables|/Script/Engine.MovementComponent|GetVelocity _charactermovement) "0, 0,100.000000"))
    (Variables|Default|SettrapDetected false)))

(event OnHearNoise(_pawnSensing)
  (params (Instigator :type Pawn%20Object%20Reference) (Location :type Vector%20%28by%20ref%29 :default "0, 0, 0") (Volume :type Float%20%28single-precision%29))
  (Development|PrintString "OnHearSensing" true true "(R=0.650000,G=0.338819,B=0.026779,A=1.000000)" 5.0))

(event OnSeePawn(_pawnSensing)
  (params (Pawn :type Pawn%20Object%20Reference))
  (CallFunction|PawnDetected)
  (Development|PrintString (Utilities|String|ToString(Vector) (Variables|/Script/Engine.MovementComponent|GetVelocity (Variables|Character|GetCharacterMovement))) true true "(R=1.000000,G=0.000000,B=0.000000,A=1.000000)"))

(event EventBeginPlay
  (Variables|Default|Set_isAppearing true)
  (Utilities|FlowControl|Delay (Class|PaperFlipbookComponent|GetFlipbookLength (Variables|Default|GetSprite)))
  (Sprite|SetFlipbook (Variables|Default|GetSprite) "/Game/Azrael/Enemy/Zombie/FlipBook/idle.idle")
  (Variables|Default|Set_isAppearing false))

(fn ConstructionScript
  (Class|Ennemy|InitEnemy))

(fn PawnDetected
  (bind _charactermovement (Variables|Character|GetCharacterMovement))
  (Development|PrintString "Hello you are detecterd")
  (Sprite|SetFlipbook (Variables|Default|GetSprite) (select (and (Variables|Default|Get_isAppearing) (> (Math|Vector|VectorLength (Transformation|GetVelocity)) 0.0)) "/Game/Azrael/Enemy/Zombie/FlipBook/idle.idle" "/Game/Azrael/Enemy/Zombie/FlipBook/walk.walk"))
  (Pawn|Input|AddMovementInput "1.000000,0.000000,0.000000" 1.0 false)
  (if (Utilities|Enum|Equal(Enum) (Variables|/Script/Engine.CharacterMovementComponent|GetMovementMode _charactermovement) "MOVE_Falling")
    _
    (else
      (Variables|/Script/Engine.MovementComponent|SetVelocity _charactermovement "500.000000, 0, 0")))
  (return))
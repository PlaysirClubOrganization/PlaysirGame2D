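; 2D flipbook zombie enemy that plays an appear delay, moves toward its facing side when it sees a pawn, and dodges traps and gaps.
; PawnSensing drives the chase, while overlap components trigger jumps over BP_Item_Pick traps and gap checks.
; At gaps, line traces and a player-height check gate a jump whose velocity derives from a sphere-traced landing actor.
; Patrol flips facing, and AnimationUpdate maps state to flipbooks, destroying the zombie after its death animation.
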(event OnComponentBeginOverlap(TrapDodge)
  (params (OtherActor :type Actor%20Object%20Reference) (OtherComp :type Primitive%20Component%20Object%20Reference) (OtherBodyIndex :type Integer) (bFromSweep :type Boolean) (SweepResult :type Hit%20Result%20Structure%20%28by%20ref%29))
  ;[0 0 0.5 0.5] When the Detector Trap is activate
  (CallFunction|TrapDetected OtherActor))

(event OnComponentEndOverlap(TrapDodge)
  (params (OtherActor :type Actor%20Object%20Reference) (OtherComp :type Primitive%20Component%20Object%20Reference) (OtherBodyIndex :type Integer)))

(event OnComponentEndOverlap(GapDodge)
  (params (OtherActor :type Actor%20Object%20Reference) (OtherComp :type Primitive%20Component%20Object%20Reference) (OtherBodyIndex :type Integer))
  ;[0.7 0.7 1] When the gap is detected
  (CallFunction|GapDetected))

(event OnSeePawn(PawnSensing)
  (params (Pawn :type Pawn%20Object%20Reference))
  ;[1 -0.3394 -0.2477 0.2342] When the Pawn Player is detected follow the player in order to kill him
  (CallFunction|PawnDetected)
  (Utilities|Time|SetTimerbyEvent (EventDispatchers|CreateEvent :!event Custom|Patrol) (Math|Random|RandomFloatinRange 1.0 3.0) true))

(event Custom|Dying
  (params (DelayTime :type Float%20%28single-precision%29))
  (Utilities|FlowControl|Delay DelayTime)
  (Actor|DestroyActor))

(event Custom|Patrol
  (|Patrolling))

(event EventBeginPlay
  (Utilities|Appear))

(event EventTick
  (params (DeltaSeconds :type Float%20%28single-precision%29)))

(fn ConstructionScript
  (Variables|Default|Set_life 100))

(fn AnimationUpdate
  (bind _sprite (Variables|Default|GetSprite))
  (bind _charactermovement (Variables|Character|GetCharacterMovement))
  (if (<= (Variables|Default|Get_life) 0)
    (Sprite|SetFlipbook _sprite "/Game/Azrael/Enemy/Zombie/Flipbook/die.die")
    (CallFunction|Dying (Class|PaperFlipbookComponent|GetFlipbookLength _sprite))
    (elif (not (Variables|Default|Get_isAppearing))
      (if (Variables|Default|Get_IsIdle)
        (Sprite|SetFlipbook (Variables|Default|GetSprite) "/Game/Azrael/Enemy/Zombie/Flipbook/idle.idle")
        (Variables|/Script/Engine.MovementComponent|SetVelocity (Variables|Character|GetCharacterMovement) "0, 0, 0")
        (elif (Variables|Default|Get_isJumping)
          (Character|Jump)
          (elif (Variables|Default|Get_isWalking)
            (Sprite|SetFlipbook (Variables|Default|GetSprite) "/Game/Azrael/Enemy/Zombie/Flipbook/walk.walk")
            (Variables|/Script/Engine.MovementComponent|SetVelocity _charactermovement "400.000000, 0, 0")
            (Pawn|Components|CharacterMovement|SetMovementMode _charactermovement "MOVE_Walking" 0)
            (elif (Variables|Default|Get_isAttacking)
              (Sprite|SetFlipbook (Variables|Default|GetSprite) "/Game/Azrael/Enemy/Zombie/Flipbook/attack.attack"))))))))

(fn CharacterUpdate)

(fn PawnDetected
  (bind _charactermovement (Variables|Character|GetCharacterMovement))
  (if (not (Variables|Default|Get_isAppearing))
    (Variables|Default|Set_playerDetected true)
    (Sprite|SetFlipbook (Variables|Default|GetSprite) "/Game/Azrael/Enemy/Zombie/Flipbook/walk.walk")
    (if (Utilities|Enum|Equal(Enum) (Variables|/Script/Engine.CharacterMovementComponent|GetMovementMode _charactermovement) "MOVE_Falling")
      (Sprite|SetFlipbook (Variables|Default|GetSprite) "/Game/Azrael/Enemy/Zombie/Flipbook/idle.idle")
      (elif (Variables|Default|GetLookAtLeft)
        (Variables|/Script/Engine.MovementComponent|SetVelocity _charactermovement "-350.000000, 0, 0")
        (else
          (Variables|/Script/Engine.MovementComponent|SetVelocity _charactermovement "350.000000, 0, 0"))))
    (return)))

(fn TrapDetected
  (params (Actor :type Actor%20Object%20Reference))
  ;[0.7 0.7 1] Check if the detected Actor is effectively a trap by casting
  (bind _output_get (Variables|Default|SetisTrapDetected (.bSuccess (Utilities|Casting|CastToBP_Item_Pick Actor))))
  (if _output_get
    ;[0.7 0.7 1] Jump to dodge the trap and change the flipbook
    (Utilities|AddVelocityJump "0.000000,0,0"))
  (return))

(fn GapDetected
  (bind _gapdodge (Variables|Default|GetGapDodge))
  (bind _gapdodge_2 (Variables|Default|GetGapDodge))
  (bind _returnvalue (Transformation|GetWorldLocation _gapdodge))
  (bind _returnvalue_2 (Transformation|GetWorldLocation _gapdodge_2))
  (if (Utilities|Enum|Equal(Enum) (Variables|/Script/Engine.CharacterMovementComponent|GetMovementMode (Variables|Character|GetCharacterMovement)) "MOVE_Walking")
    (if (Variables|Default|GetLookAtLeft)
      (bind _returnvalue_3 (Collision|LineTraceByChannel (+ _returnvalue "-20.000000, 0, 0") (+ _returnvalue "-100.000000, 0, 0") "TraceTypeQuery1" false 0 "ForDuration"))
      (else
        (bind _returnvalue_4 (Collision|LineTraceByChannel (+ _returnvalue_2 "20.000000, 0, 0") (+ _returnvalue_2 "100.000000, 0, 0") "TraceTypeQuery1" false 0 "ForDuration"))))
    (if (or _returnvalue_4 _returnvalue_3)
      _
      (else
        (Utilities|CheckZpositionPlayer
          (:true
            (Pawn|Components|CharacterMovement|SetMovementMode (Variables|Character|GetCharacterMovement) "MOVE_Flying" 0)
            (bind _velocity (CallFunction|GetJumpZVelocity))
            (Utilities|AddVelocityJump _velocity))
          (:false
            _))))
    (Pawn|Components|CharacterMovement|SetMovementMode (Variables|Character|GetCharacterMovement) "MOVE_Falling" 0))
  (return))

(fn GetJumpZVelocity
  (bind _returnvector (CallFunction|GetVectorfromRotation (Transformation|GetActorLocation) "200.000000, 0,50.000000"))
  (bind _returnvector_2 (CallFunction|GetVectorfromRotation _returnvector "0,1.000000, 0"))
  (bind (_outhit _returnvalue) (Class|KismetSystemLibrary|SphereTraceSingleNEW _returnvector _returnvector_2 1e+02 "TraceTypeQuery1" false 0 "Persistent" true))
  (if _returnvalue
    (if (< (.z (- (Transformation|GetActorLocation (.hitactor _outhit)) (Transformation|GetActorLocation))) 0.0)
      (return (Math|Vector|MakeVector 0.0 0.0 (* (Math|Float|Absolute(Float) (.z (- (Transformation|GetActorLocation (.hitactor _outhit)) (Transformation|GetActorLocation)))) 12.0)))
      (else
        (return (Math|Vector|MakeVector (* (/ 3.0 (Math|Float|Sqrt (Math|Float|Absolute(Float) (.x (- (Transformation|GetActorLocation (.hitactor _outhit)) (Transformation|GetActorLocation)))))) -1e+01) 0.0 (- (* (Math|Float|Absolute(Float) (.z (- (Transformation|GetActorLocation (.hitactor _outhit)) (Transformation|GetActorLocation)))) 8.0) (Math|Float|Sqrt (Math|Float|Absolute(Float) (.x (- (Transformation|GetActorLocation (.hitactor _outhit)) (Transformation|GetActorLocation))))))))))
    (else
      (return ""))))

(fn GetVectorfromRotation
  (params (VectorIn :type Vector) (VectorPlus :type Vector))
  (if (Variables|Default|GetLookAtLeft)
    (return (- VectorIn VectorPlus))
    (else
      (return (+ VectorIn VectorPlus)))))
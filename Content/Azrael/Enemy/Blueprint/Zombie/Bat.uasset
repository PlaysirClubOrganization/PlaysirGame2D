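; Bat enemy pawn that lunges at the player when its PawnSensing component spots a pawn.
; On sight, it eases the capsule toward player 0's current location over a time inversely proportional to distance, so farther targets mean shorter moves.
; The Tick distance check does nothing, and the look-at rotation logic is disconnected.
; IsPlayerLost compares two counters to detect a stalled count, but nothing here calls it.
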(event OnSeePawn(PawnSensing)
  (params (Pawn :type Pawn%20Object%20Reference))
  (bind _returnvalue (Game|Player|GetPlayerPawn 0))
  (Components|MoveComponentTo (Variables|Default|GetCapsuleComponent) (Transformation|GetActorLocation _returnvalue) "0, 0, 0" false true (/ 15.0 (Transformation|GetDistanceTo _returnvalue))))

(event EventBeginPlay)

(event EventTick
  (params (DeltaSeconds :type Float%20%28single-precision%29))
  (if (> (Transformation|GetDistanceTo (Game|Player|GetPlayerPawn 0)) 1.5e+02)
    _))

(fn ConstructionScript)

(fn IsPlayerLost
  (if (== (Variables|Default|Getcount1) (Variables|Default|Getcount2))
    (Variables|Default|Setcount1 1)
    (Variables|Default|Setcount2 0)
    (return true)
    (else
      (Variables|Default|Setcount2 (Variables|Default|Getcount1))
      (return false))))
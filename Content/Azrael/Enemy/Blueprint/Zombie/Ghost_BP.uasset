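; Ghost enemy Blueprint in the zombie enemy folder that homes in on the player.
; Unless it is appearing, each Tick starts a short eased capsule move toward player pawn 0's location, with yaw computed from the player toward the ghost.
; Attack prints a debug string, then calls the parent attack.
; IsPlayerLost reports true and resets two counters when they match, otherwise it syncs them.
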(event EventBeginPlay)

(event EventTick
  (params (DeltaSeconds :type Float%20%28single-precision%29))
  (bind _returnvalue (Game|Player|GetPlayerPawn 0))
  (bind _returnvalue_2 (Transformation|GetActorLocation _returnvalue))
  (if (not (Variables|Default|Get_isAppearing))
    (Components|MoveComponentTo (Variables|Default|GetCapsuleComponent) _returnvalue_2 (Math|Rotator|MakeRotator 0.0 0.0 (.yaw (Math|Rotator|FindLookatRotation _returnvalue_2 (Transformation|GetActorLocation)))) true true 0.1)))

(event EventAttack
  (Development|PrintString "Attack")
  (|CallParentFunction))

(fn ConstructionScript)

(fn IsPlayerLost
  (if (== (Variables|Default|Getcount1) (Variables|Default|Getcount2))
    (Variables|Default|Setcount1 1)
    (Variables|Default|Setcount2 0)
    (return true)
    (else
      (Variables|Default|Setcount2 (Variables|Default|Getcount1))
      (return false))))
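; Vampire enemy: a Paper2D side-scrolling character that plays an appearance delay on spawn and runs when it sees a pawn.
; Pawn sensing sets flipbook and forward velocity, while a TrapDodge overlap jumps over BP_Item_Pick traps.
; AnimationUpdate maps life and state flags to flipbooks, movement and delayed destruction, but nothing here calls it.
; Gap dodging is unwired: its overlap event is empty and GapDetected is never called.
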(event OnComponentBeginOverlap(TrapDodge)
  (params (OtherActor :type Actor%20Object%20Reference) (OtherComp :type Primitive%20Component%20Object%20Reference) (OtherBodyIndex :type Integer) (bFromSweep :type Boolean) (SweepResult :type Hit%20Result%20Structure%20%28by%20ref%29))
  ;[0 0 0.5 0.5] When the Detector Trap is activate
  (CallFunction|TrapDetected OtherActor))

(event OnComponentEndOverlap(GapDodge)
  (params (OtherActor :type Actor%20Object%20Reference) (OtherComp :type Primitive%20Component%20Object%20Reference) (OtherBodyIndex :type Integer))
  ;[0.7 0.7 1] When the gap is detected
)

(event OnSeePawn(PawnSensing)
  (params (Pawn :type Pawn%20Object%20Reference))
  ;[1 -0.3394 -0.2477 0.2342] When the Pawn Player is detected follow the player in order to kill him
  (CallFunction|PawnDetected))

(event Custom|Dying
  (params (DelayTime :type Float%20%28single-precision%29))
  (Utilities|FlowControl|Delay DelayTime)
  (Actor|DestroyActor))

(event EventBeginPlay
  (Utilities|Appear))

(event Collision|EventActorBeginOverlap
  (params (OtherActor :type Actor%20Object%20Reference)))

(event EventTick
  (params (DeltaSeconds :type Float%20%28single-precision%29)))

(fn ConstructionScript
  (Variables|Default|Set_life 100))

(fn AnimationUpdate
  (bind _sprite (Variables|Default|GetSprite))
  (bind _charactermovement (Variables|Character|GetCharacterMovement))
  (if (<= (Variables|Default|Get_life) 0)
    (Sprite|SetFlipbook _sprite "/Game/Azrael/Enemy/Zombie/Flipbook/die.die")
    (CallFunction|Dying (Class|PaperFlipbookComponent|GetFlipbookLength _sprite))
    (elif (not (Variables|Default|Get_isAppearing))
      (if (Variables|Default|Get_IsIdle)
        (Sprite|SetFlipbook (Variables|Default|GetSprite) "/Game/Azrael/Enemy/Zombie/Flipbook/idle.idle")
        (Variables|/Script/Engine.MovementComponent|SetVelocity (Variables|Character|GetCharacterMovement) "0, 0, 0")
        (elif (Variables|Default|Get_isJumping)
          (Character|Jump)
          (elif (Variables|Default|Get_isWalking)
            (Sprite|SetFlipbook (Variables|Default|GetSprite) "/Game/Azrael/Enemy/Zombie/Flipbook/walk.walk")
            (Variables|/Script/Engine.MovementComponent|SetVelocity _charactermovement "400.000000, 0, 0")
            (Pawn|Components|CharacterMovement|SetMovementMode _charactermovement "MOVE_Walking" 0)
            (elif (Variables|Default|Get_isAttacking)
              (Sprite|SetFlipbook (Variables|Default|GetSprite) "/Game/Azrael/Enemy/Zombie/Flipbook/attack.attack"))))))))

(fn CharacterUpdate)

(fn PawnDetected
  (bind _charactermovement (Variables|Character|GetCharacterMovement))
  (Development|PrintString "Hello you are detecterd")
  (Sprite|SetFlipbook (Variables|Default|GetSprite) (select (and (Variables|Default|Get_isAppearing) (> (Math|Vector|VectorLength (Transformation|GetVelocity)) 0.0)) "/Game/Azrael/Enemy/Zombie/Flipbook/idle.idle" "/Game/Azrael/Enemy/Zombie/Flipbook/walk.walk"))
  (if (Utilities|Enum|Equal(Enum) (Variables|/Script/Engine.CharacterMovementComponent|GetMovementMode _charactermovement) "MOVE_Falling")
    _
    (else
      (Variables|/Script/Engine.MovementComponent|SetVelocity _charactermovement "700.000000, 0, 0")))
  (return))

(fn TrapDetected
  (params (Actor :type Actor%20Object%20Reference))
  ;[0.7 0.7 1] Check if the detected Actor is effectively a trap by casting
  (bind _output_get (Variables|Default|SetisTrapDetected (.bSuccess (Utilities|Casting|CastToBP_Item_Pick Actor))))
  (if _output_get
    ;[0.7 0.7 1] Jump to dodge the trap and change the flipbook
    (Character|Jump)
    (Sprite|SetFlipbook (Variables|Default|GetSprite) "/Game/Azrael/Enemy/Zombie/Flipbook/idle.idle")
    (Variables|/Script/Engine.MovementComponent|SetVelocity (Variables|Character|GetCharacterMovement) (Math|Vector|MakeVector 3e+02 0.0 0.0)))
  (return))

(fn GapDetected
  (bind _charactermovement (Variables|Character|GetCharacterMovement))
  (if (Variables|Default|GetisTrapDetected)
    _
    (else
      (Character|Jump)
      (Variables|/Script/Engine.MovementComponent|SetVelocity _charactermovement (+ (Variables|/Script/Engine.MovementComponent|GetVelocity _charactermovement) "0, 0,100.000000"))
      (Variables|Default|SetisTrapDetected false)))
  (return))
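; Item Blueprint that acts as a kill trigger for the player's alien hero, restarting the current level on contact.
; On overlap, it calls DestroyOnActor with AlienHero_BP as the target class and the overlapping actor as the one to destroy.
; When that succeeds, it calls RestartGame on the game mode, then reopens the level named "Level" plus the level value in AlienHeroGameMode's SaveMode.
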(event EventBeginPlay)

(event EventActorBeginOverlap
  (params (OtherActor :type Actor%20Object%20Reference))
  (|CallParentFunction OtherActor)
  (bind _suceeddestroy (CallFunction|DestroyonActor "/Game/Azrael/Gameplay/AlienHero_BP.AlienHero_BP_C" OtherActor OtherActor))
  (if _suceeddestroy
    (Class|GameMode|RestartGame (Game|GetGameMode))
    (CallFunction|ReloadCurrentLevel)))

(event EventTick
  (params (DeltaSeconds :type Float%20%28single-precision%29)))

(fn ConstructionScript
  (|CallParentFunction))

(fn ReloadCurrentLevel
  (Game|OpenLevel(byName) (Utilities|String|StringToName (Utilities|String|Append "Level" (Utilities|String|ToString(Integer) (Variables|/Game/Azrael/Gameplay/BP_SaveGame.BP_SaveGame_C|GetLevel (Variables|/Game/Azrael/Gameplay/AlienHeroGameMode.AlienHeroGameMode_C|GetSaveMode (.AsAlien%20Hero%20Game%20Mode (Utilities|Casting|CastToAlienHeroGameMode (Game|GetGameMode)))))))))
  (return))
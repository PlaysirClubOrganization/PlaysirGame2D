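; BP_Projectile is a projectile actor that travels horizontally along the world X axis.
; Its construction script reads the yaw of the pawn sprite held by AlienHeroGameMode, sets a positive or negative Direction from that facing, and prints the yaw.
; Tick moves the actor by a fixed step in that direction every frame, without delta-time scaling, collision handling or lifetime logic in the graph.
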(event EventBeginPlay)

(event EventActorBeginOverlap
  (params (OtherActor :type Actor%20Object%20Reference)))

(event EventTick
  (params (DeltaSeconds :type Float%20%28single-precision%29))
  (bind _returnvalue (Transformation|GetActorLocation))
  (Transformation|SetActorLocation (Math|Vector|MakeVector (+ (* (Variables|Default|Getdirection) 12.0) (.x _returnvalue)) (.y _returnvalue) (.z _returnvalue)) false false))

(fn ConstructionScript
  (bind _returnvalue (Game|GetGameMode))
  (bind _asalien_hero_game_mode (Utilities|Casting|CastToAlienHeroGameMode _returnvalue))
  (bind _pawn (Variables|/Game/Azrael/Gameplay/AlienHeroGameMode.AlienHeroGameMode_C|GetPawn _asalien_hero_game_mode))
  (bind _sprite (Variables|/Script/Paper2D.PaperCharacter|GetSprite _pawn))
  (bind _relativerotation (Variables|/Script/Engine.SceneComponent|GetRelativeRotation _sprite))
  (if (== 0.0 (.yaw _relativerotation))
    (Variables|Default|Setdirection 2)
    (else
      (Variables|Default|Setdirection -2)))
  (Development|PrintString (Utilities|String|ToString(Float) (.yaw _relativerotation))))
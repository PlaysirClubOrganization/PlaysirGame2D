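; SpiritHero_BP is a spirit companion that follows the AlienHero_BP player pawn, cached on BeginPlay.
; MoveToTarget runs every Tick, gliding the capsule with MoveComponentTo.
; The player sprite's yaw selects the TargetRight or TargetLeft anchor and flips the spirit's yaw to suit.
; While MasteringTime is true, it instead moves quickly to a point above the player with zero rotation; the flag is not set here.
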(event EventBeginPlay
  (bind _asalien_hero_bp (Utilities|Casting|CastToAlienHero_BP (Game|Player|GetPlayerPawn 0)))
  (Variables|Default|SetPlayer _asalien_hero_bp)
  (Utilities|MovetoTarget))

(event EventTick
  (params (DeltaSeconds :type Float%20%28single-precision%29))
  (Utilities|MovetoTarget))

(fn ConstructionScript)
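; Grapple actor that shows a rope effect between itself and an anchor target.
; On BeginPlay it passes itself and the anchor to the Rope component as source and target actor parameters.
; Each tick it checks its distance to a valid anchor and destroys itself once close enough.
; The graph contains no movement logic of its own.
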(event EventBeginPlay
  ;[1 1 1] Attent de commentaire
  (Effects|Components|ParticleSystem|SetActorParameter (Variables|Default|GetRope) "GrappleTarget" (Variables|Default|GetAnchorTarget))
  (Effects|Components|ParticleSystem|SetActorParameter (Variables|Default|GetRope) "GrappleSource" self))

(event Collision|EventActorBeginOverlap
  (params (OtherActor :type Actor%20Object%20Reference)))

(event EventTick
  (params (DeltaSeconds :type Float%20%28single-precision%29))
  (bind _anchortarget (Variables|Default|GetAnchorTarget))
  ;[1 1 1] Attent de commentaire
  (Utilities|IsValid _anchortarget
    (:Is%20Valid
      (if (< (Transformation|GetDistanceTo _anchortarget) 1e+02)
        (Actor|DestroyActor)))))

(fn ConstructionScript)
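; AlienHero_BP is the playable side-scrolling hero, with walking, jumping, ladder climbing and a timed attack.
; BeginPlay adds the coin HUD, then loads or creates the save object.
; Climbing uses Flying mode with set vertical velocity, freezing the hero and animation on release, while jumping restores Walking.
; Attacking blocks movement for the current sprite's length; BP_Keyhold calls LockDestroyed, and a gamepad key spawns test ghosts.
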(event Custom|LockDestroyed
  ;[1 1 1] Event : destroying the lock, called in BP_Keyhold
  (Variables|Default|SetLock true))

(event EventBeginPlay
  ;[0.2636 0.1327 1] Begin Play : Initialisation of the save game object and displaying the caracter 's widget
  (bind _returnvalue (UserInterface|CreateWidget "/Game/Azrael/Blueprint/HUD/HUD_Coin.HUD_Coin_C"))
  (UserInterface|Viewport|AddtoViewport _returnvalue 0)
  (bind _returnvalue_2 (SaveGame|DoesSaveGameExist "PlaysirGame"))
  (if _returnvalue_2
    (bind _returnvalue_3 (SaveGame|LoadGamefromSlot "PlaysirGame"))
    (bind _output_get (Variables|Default|SetSaver (.AsBP%20Save%20Game (Utilities|Casting|CastToBP_SaveGame _returnvalue_3))))
    (Class|AbstractPlayer|LoadData _output_get)
    (else
      (bind _returnvalue_4 (SaveGame|CreateSaveGameObject "/Game/Azrael/Gameplay/BP_SaveGame.BP_SaveGame_C"))
      (Variables|Default|SetSaver (.AsBP%20Save%20Game (Utilities|Casting|CastToBP_SaveGame _returnvalue_4))))))

(event Input|ActionEvents|InputActionPlayerAttack
  (params (Key :type Key%20Structure :default "AnyKey"))
  ;[1 1 1] AttackPlayer
  (:Pressed
    (if (not (Variables|Default|Get_isDead))
      (Variables|Default|Set_isAttacking true)
      (Utilities|FlowControl|Delay (Class|AzraelCharacter|GetCurrentSpriteLength))
      (Variables|Default|Set_isAttacking false))))

(event Input|ActionEvents|InputActionclimb
  (params (Key :type Key%20Structure :default "AnyKey"))
  ;[1 1 1] Handle Climb Movement
  (:Pressed
    ;;[1 0.008092 0] Checking if the character is in the ladder
    (if (Variables|Default|GetcanClimb)
      (Action|Climb true) ; Climb Up
    ))
  (:Released
    (if (Variables|Default|GetcanClimb)
      (CallFunction|StopClimbing))))

(event Input|ActionEvents|InputActionJump
  (params (Key :type Key%20Structure :default "AnyKey"))
  ;[1 1 1] Handle Jump (if he is climbing he can jump)
  (:Pressed
    (if (Variables|Default|GetcanClimb)
      (Pawn|Components|CharacterMovement|SetMovementMode (Variables|Character|GetCharacterMovement) "MOVE_Walking" 0))
    (Character|Jump)))

(event Input|AxisEvents|InputAxisMoveRight
  (params (AxisValue :type Float%20%28single-precision%29))
  (bind _sprite (Variables|Default|GetSprite))
  ;[1 1 1] Handle movement
  (if (not (Variables|Default|Get_isAttacking))
    (if (> AxisValue 0.0)
      (Transformation|SetRelativeRotation _sprite "0,180.000000, 0" false false)
      (Pawn|Input|AddMovementInput "1.000000, 0, 0" AxisValue false :!label _label)
      (elif (< AxisValue 0.0)
        (Transformation|SetRelativeRotation _sprite "0.000000,0.000000,0.000000" false false)
        (goto _label)))))

(event Input|GamepadEvents|GamepadFaceButtonRight
  (params (Key :type Key%20Structure :default "AnyKey"))
  ;[1 1 1] Spawn Enemy ( for test gameplay)
  (:Pressed
    (Game|SpawnActorfromClass "/Game/Azrael/Enemy/Blueprint/Zombie/Ghost_BP.Ghost_BP_C" (Math|Transform|MakeTransform (Math|Vector|MakeVector 2e+03 0.0 5e+02) "0, 0, 0" "0.100000,1.000000,0.100000") "Undefined" 0 2.0 0)))

(event Input|KeyboardEvents|Down
  (params (Key :type Key%20Structure :default "AnyKey"))
  ;[1 1 1] Handle Climb Movement
  (:Pressed
    ;;[1 0.008092 0] Checking if the character is in the ladder
    (if (Variables|Default|GetcanClimb)
      (Action|Climb false) ; Climb Down
    ))
  (:Released
    (if (Variables|Default|GetcanClimb)
      (CallFunction|StopClimbing))))

(event Input|TouchEvents|InputTouch
  (params (Location :type Vector) (FingerIndex :type ETouchIndex%20Enum))
  ;[1 1 1] Handle Jump (if he is climbing he can jump)
  (:Pressed
    (if (Variables|Default|GetcanClimb)
      (Pawn|Components|CharacterMovement|SetMovementMode (Variables|Character|GetCharacterMovement) "MOVE_Walking" 0))
    (Character|Jump)))

(fn ConstructionScript)

(fn Climb
  (params (isClimbUp :type Boolean))
  ;[0.1037 1 0.1853] Adding the movement input through the Z axis and setting the character in flying mode
  (Pawn|Components|CharacterMovement|SetMovementMode (Variables|Character|GetCharacterMovement) "MOVE_Flying" 0)
  (Pawn|Input|AddMovementInput (Math|Vector|MakeVector 0.0 0.0 (.Z (Math|Vector|BreakVector (Math|Rotator|GetRotationXVector (Math|Rotator|MakeRotator 0.0 (.Pitch (Math|Rotator|BreakRotator (Pawn|GetControlRotation :!class /Script/Engine.Pawn))) 0.0))))) 1.0 true)
  ;[1 0.8838 0.1019] Giving the velocity to the actor and playing the sprite animation
  (Variables|/Script/Engine.MovementComponent|SetVelocity (Variables|Character|GetCharacterMovement) (|CreateVectorvelocityaccordingtotheboolparamerteristheclimbactionisUporDown isClimbUp))
  (Variables|Default|SetisClimbing true)
  (Components|Timeline|SetPlayRate (Variables|Default|GetSprite) 1.0))

(fn StopClimbing
  ;[0 1 0.08696] Stoping the animation and set the velocity at null. The character is in flying mode so he will be static in the air
  (Variables|Default|SetisClimbing false)
  (Variables|/Script/Engine.MovementComponent|SetVelocity (Variables|Character|GetCharacterMovement) "0, 0,0.000000")
  (Components|Timeline|SetPlayRate (Variables|Default|GetSprite) 0.0)
  (return))